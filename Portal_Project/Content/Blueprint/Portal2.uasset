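; Second portal of a linked pair that teleports overlapping actors to Portal 1, sharing state through FirstPersonCharacter.
; Tick publishes its location, shows Portal 1's render-target material once that portal exists, and rotates Portal2View from player camera rotation and Portal 1's axis-aligned facing.
; New placement briefly moves the overlap volume away and back.
; A CanTeleport cooldown limits re-triggering; player rotation and velocity functions are empty stubs.
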(event OnComponentBeginOverlap(TeleportOnOverlap)
  (params (OverlappedComponent :type Primitive%20Component%20Object%20Reference) (OtherActor :type Actor%20Object%20Reference) (OtherComp :type Primitive%20Component%20Object%20Reference) (OtherBodyIndex :type Integer) (bFromSweep :type Boolean) (SweepResult :type Hit%20Result%20Structure%20%28by%20ref%29))
  ;[1 1 1] Teleport Player On Overlap
  (if (Variables|Default|GetIsSecondPortalMade)
    (Utilities|Casting|CastToFirstPersonCharacter OtherActor
      (:then
        (Variables|Default|SetIsPlayer true))
      (:CastFailed
        (Variables|Default|SetIsPlayer false)))
    (Variables|Default|SetPortal2ForwarVector (Variables|/Game/FirstPersonBP/Blueprints/FirstPersonCharacter.FirstPersonCharacter_C|GetPortal2ForwardVector (Variables|Default|GetCast%20To%20FPC)))
    (if (Variables|/Game/FirstPersonBP/Blueprints/FirstPersonCharacter.FirstPersonCharacter_C|GetCanTeleport (Variables|Default|GetCast%20To%20FPC))
      (Variables|/Game/FirstPersonBP/Blueprints/FirstPersonCharacter.FirstPersonCharacter_C|SetCanTeleport (Variables|Default|GetCast%20To%20FPC) false)
      (Transformation|SetActorLocation OtherActor (Variables|/Game/FirstPersonBP/Blueprints/FirstPersonCharacter.FirstPersonCharacter_C|GetPortal1 (Variables|Default|GetCast%20To%20FPC)) false true)
      (if (Variables|Default|GetIsPlayer)
        (CallFunction|SetPlayerRotation)
        (CallFunction|SetPlayerVelocity))
      (Utilities|FlowControl|Delay 0.2)
      (if (not (Variables|/Game/FirstPersonBP/Blueprints/FirstPersonCharacter.FirstPersonCharacter_C|GetCanTeleport (Variables|Default|GetCast%20To%20FPC)))
        (Variables|/Game/FirstPersonBP/Blueprints/FirstPersonCharacter.FirstPersonCharacter_C|SetCanTeleport (Variables|Default|GetCast%20To%20FPC) true)))))

(event Custom|ChangeOverlapPosition
  (Variables|Default|SetCollisionOriginalLocation (Transformation|GetWorldLocation (Variables|Default|GetTeleportOnOverlap)))
  (Transformation|SetWorldLocation (Variables|Default|GetTeleportOnOverlap) (Variables|Default|GetCollisionRandomLocation) false true)
  (Utilities|FlowControl|Delay 0.1)
  (Transformation|SetWorldLocation (Variables|Default|GetTeleportOnOverlap) (Variables|Default|GetCollisionOriginalLocation) false true)
  (if (Variables|Default|GetFirstRun)
    (Variables|Default|SetFirstRun false)
    (else
      (Variables|/Game/FirstPersonBP/Blueprints/FirstPersonCharacter.FirstPersonCharacter_C|SetNewlyCreatedPortal2 (Variables|Default|GetCast%20To%20FPC) false))))

(event EventBeginPlay
  (bind _asfirst_person_character (Utilities|Casting|CastToFirstPersonCharacter (Game|GetPlayerCharacter 0)))
  (Variables|Default|SetCast%20To%20FPC _asfirst_person_character)
  (Variables|Default|SetCollisionOriginalLocation (Transformation|GetWorldLocation (Variables|Default|GetTeleportOnOverlap)))
  (Transformation|SetWorldLocation (Variables|Default|GetTeleportOnOverlap) (Variables|Default|GetCollisionRandomLocation) false true)
  (Utilities|FlowControl|Delay 0.1)
  (Transformation|SetWorldLocation (Variables|Default|GetTeleportOnOverlap) (Variables|Default|GetCollisionOriginalLocation) false true)
  (if (Variables|Default|GetFirstRun)
    (Variables|Default|SetFirstRun false)
    (else
      (Variables|/Game/FirstPersonBP/Blueprints/FirstPersonCharacter.FirstPersonCharacter_C|SetNewlyCreatedPortal2 (Variables|Default|GetCast%20To%20FPC) false))))

(event Collision|EventActorBeginOverlap
  (params (OtherActor :type Actor%20Object%20Reference)))

(event EventTick
  (params (DeltaSeconds :type Float%20%28single-precision%29))
  ;[1 1 1] Get If Portal 1 Has Been Created
  (Variables|/Game/FirstPersonBP/Blueprints/FirstPersonCharacter.FirstPersonCharacter_C|SetPortal2 (Variables|Default|GetCast%20To%20FPC) (Transformation|GetWorldLocation (Variables|Default|GetDefaultSceneRoot)))
  (if (Math|Vector|Equal(Vector) (Variables|/Game/FirstPersonBP/Blueprints/FirstPersonCharacter.FirstPersonCharacter_C|GetPortal1 (Variables|Default|GetCast%20To%20FPC)) "0, 0, 0" 1.0)
    (Rendering|Material|SetMaterial (Variables|Default|GetPlane) 0 "/Game/Blueprint/NoPortal1Created_Inst.NoPortal1Created_Inst")
    (else
      (Rendering|Material|SetMaterial (Variables|Default|GetPlane) 0 "/Game/Blueprint/Portal1_RT_Mat.Portal1_RT_Mat")
      (Variables|Default|SetIsSecondPortalMade true)
      (if (Variables|/Game/FirstPersonBP/Blueprints/FirstPersonCharacter.FirstPersonCharacter_C|GetNewlyCreatedPortal2 (Variables|Default|GetCast%20To%20FPC))
        (CallFunction|ChangeOverlapPosition))
      (CallFunction|SetRenderTargetRotation))))

(fn ConstructionScript)

(fn SetPlayerVelocity)

(fn SetPlayerRotation)

(fn ResetMaxAcceleration)

(fn SetVelocityAccordingtoForwardVector)

(fn SetPortal1LocationonCall)

(fn SetRenderTargetRotation
  (Variables|Default|SetPlayerRotation (Transformation|GetWorldRotation (Variables|/Script/Engine.PlayerCameraManager|GetTransformComponent (Game|GetPlayerCameraManager 0))))
  (Variables|Default|SetPortal1ForwardVector (Variables|/Game/FirstPersonBP/Blueprints/FirstPersonCharacter.FirstPersonCharacter_C|GetPortal1ForwardVector (Variables|Default|GetCast%20To%20FPC)))
  ;[1 1 1] If Portal 1 Is Spawned at -X Axis
  (if (== (.x (Variables|Default|GetPortal1ForwardVector)) 1.0)
    (Transformation|SetRelativeRotation (Variables|Default|GetPortal2View) (Math|Rotator|MakeRotator 0.0 (* 1 (.pitch (Variables|Default|GetPlayerRotation))) (* -1 (- 1.8e+02 (.yaw (Variables|Default|GetPlayerRotation))))) false false)
    (else
      ;[1 1 1] If Portal 1 Is Spawned At +X Axis
      (if (== (.x (Variables|Default|GetPortal1ForwardVector)) -1.0)
        (Transformation|SetRelativeRotation (Variables|Default|GetPortal2View) (Math|Rotator|MakeRotator 0.0 (.pitch (Variables|Default|GetPlayerRotation)) (.yaw (Variables|Default|GetPlayerRotation))) false false)
        (else
          ;[1 1 1] If Portal 1 Is Spawned At -Y Axis
          (if (== (.y (Variables|Default|GetPortal1ForwardVector)) 1.0)
            (Transformation|SetRelativeRotation (Variables|Default|GetPortal2View) (Math|Rotator|MakeRotator 0.0 (* 1 (.pitch (Variables|Default|GetPlayerRotation))) (* -1 (- -9e+01 (.yaw (Variables|Default|GetPlayerRotation))))) false false)
            (else
              ;[1 1 1] If Portal 1 Is Spawned At +Y Axis
              (if (== (.y (Variables|Default|GetPortal1ForwardVector)) -1.0)
                (Transformation|SetRelativeRotation (Variables|Default|GetPortal2View) (Math|Rotator|MakeRotator 0.0 (.pitch (Variables|Default|GetPlayerRotation)) (* -1 (- 9e+01 (.yaw (Variables|Default|GetPlayerRotation))))) false false)))))))))